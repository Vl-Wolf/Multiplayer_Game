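; Networked enemy character with a suicide explosion attack: a multicast applies radial falloff damage, spawns FX and destroys the actor.
; Incoming damage feeds the TTHealth component, whose death event makes the server multicast the last death montage.
; On authority, death also stops movement, unpossesses, sets a lifespan, clears the CanMove/CanAttack flags and ragdolls on montage blend-out, while remotes only play the montage.
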(event `self.TT_Health.OnDead`
  (bind _deathmontage (`self.DeathMontage`))
  (`/Engine/EditorBlueprintResources/ActorMacros.Switch Has Authority`
    (:`Authority`
      (bind _output_get (set `self.SelectedDeadMontage` (`|GetArrayItem` _deathmontage (- (`KismetArrayLibrary.Array_Length` _deathmontage) 1))))
      (`self.DeadEvent_Multicast` _output_get))))

(event `self.ReceiveAnyDamage`
  (params (Damage :type "Float (single-precision)") (DamageType :type "DamageType Object Reference") (InstigatedBy :type "Controller Object Reference") (DamageCauser :type "Actor Object Reference"))
  (`TT_HealthComponent.ChangeHealthValue_OnServer` (`self.TT_Health`) (* Damage -1.0)))

(event `DeadEvent_Multicast`
  (params (SelectedDead :type "AnimMontage Object Reference"))
  (`/Engine/EditorBlueprintResources/ActorMacros.Switch Has Authority`
    (:`Authority`
      (`|PlayMontage` (`self.Mesh`) SelectedDead
        (:`then`
          (`self.DeadEvent`))
        (:`OnBlendOut`
          (`self.EnableRagdoll`))))
    (:`Remote`
      (`self.PlayAnimMontage` SelectedDead))))

(event `EnableRagdoll`
  (bind _mesh (`self.Mesh`))
  (`PrimitiveComponent.SetCollisionResponseToChannel` (`self.CapsuleComponent`) "ECC_Pawn" "ECR_Ignore")
  (`PrimitiveComponent.SetCollisionEnabled` _mesh "PhysicsOnly")
  (`PrimitiveComponent.SetCollisionProfileName` _mesh "PhysicsActor" true)
  (`PrimitiveComponent.SetSimulatePhysics` _mesh true)
  (`PrimitiveComponent.SetCollisionObjectType` _mesh "ECC_PhysicsBody"))

(event `/Game/Blueprint/Enemy/BPI_Combat.Attack`
  (`self.SetStateAttack` false)
  (`self.Attack_Multicast`))

(event `Attack_Multicast`
  (`GameplayStatics.ApplyRadialDamageWithFalloff` :`BaseDamage` 40.0 :`MinimumDamage` 20.0 :`Origin` (`self.K2_GetActorLocation`) :`DamageInnerRadius` (`self.ExplosionMinRadius`) :`DamageOuterRadius` (`self.ExplosionMaxRadius`) :`DamageFalloff` 1.0 :`DamageCauser` null :`InstigatedByController` null)
  (`NiagaraFunctionLibrary.SpawnSystemAtLocation` (`self.ExplosionFX`) (`self.K2_GetActorLocation`) (`self.K2_GetActorRotation`))
  (`self.SetStateAttack` true)
  (`self.K2_DestroyActor`))

(fn `CanAttack`
  (returns (bIsCanAttack :type Boolean))
  (return (`self.Can Attack`)))

(fn `CanMove`
  (returns (bIsCanMove :type Boolean))
  (return (`self.Can Move`)))

(fn `DeadEvent`
  (`MovementComponent.StopMovementImmediately` (`self.CharacterMovement`))
  (`Controller.UnPossess` (`self.GetController`))
  (`self.SetLifeSpan` 10.0)
  (`self.SetStateMovement` false)
  (`self.SetStateAttack` false))

(fn `SetStateAttack`
  (params (bCanAttack :type Boolean))
  (set `self.Can Attack` bCanAttack))

(fn `SetStateMovement`
  (params (bCanMove :type Boolean))
  (set `self.Can Move` bCanMove))

(fn `UserConstructionScript`)