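; BP_PickUp_Health is a health pickup that changes the health of a BP_Character that overlaps it.
; It extends the parent pickup's overlap event, resolving the character from the owner of the passed Inventory component.
; When current health is below 100, it applies ChangeValue through the Health component's server call and then reports pickup success, so characters at full health do not trigger it.
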(event `self.OverlapCharacter`
  (params (Inventory :type "TT_InventoryComponent Object Reference"))
  (`parent.OverlapCharacter` Inventory)
  (bind _asbp_character (cast `/Game/Blueprint/Character/BP_Character` (`ActorComponent.GetOwner` Inventory)))
  (bind _health (`TTCharacter.Health` _asbp_character))
  (bind _returnvalue (`TT_HealthComponent.GetCurrentHealth` _health))
  (if (< _returnvalue 100.0)
    (`TT_HealthComponent.ChangeHealthValue_OnServer` _health (`self.Change Value`))
    (`self.PickUpSucces`)))

(fn `UserConstructionScript`
  (`parent.UserConstructionScript`))