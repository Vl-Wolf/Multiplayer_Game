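; Ammo pickup actor that grants ammunition of a configured weapon type to an overlapping character.
; On BeginPlay it swaps its Niagara effect to the asset matching the weapon type, Rifle or Railgun.
; On character overlap it asks the inventory whether that ammo can be taken, then adds the count and triggers the inherited pickup-success handling.
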(event `self.ReceiveBeginPlay`
  (`self.InitActor`))

(event `self.OverlapCharacter`
  (params (Inventory :type "TT_InventoryComponent Object Reference"))
  (bind _weapontype (`self.WeaponType`))
  (`parent.OverlapCharacter` Inventory)
  (bind _returnvalue (`TT_InventoryComponent.CheckCanTakeAmmo` Inventory _weapontype))
  (if _returnvalue
    (`TT_InventoryComponent.AmmoSlotChangeValue` Inventory _weapontype (`self.Count`))
    (`self.PickUpSucces`)))

(fn `InitActor`
  (bind _returnvalue (select `EWeaponType` (`self.WeaponType`) :`RifleType` "/Game/sA_Megapack_v1/sA_PickupSet_1/Fx/NiagaraSystems/NS_Pickup_1.NS_Pickup_1" :`RailgunType` "/Game/sA_Megapack_v1/sA_PickupSet_1/Fx/NiagaraSystems/NS_Pickup_2.NS_Pickup_2" :!type "NiagaraSystem Object Reference"))
  (`/Engine/EditorBlueprintResources/StandardMacros.IsValid` _returnvalue
    (:`Is Valid`
      (`NiagaraComponent.SetAsset` (`self.Niagara`) _returnvalue true))))

(fn `UserConstructionScript`
  (`parent.UserConstructionScript`))